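; BP_HandsPlayerController is a player controller that lets keys 1 and 2 rotate a table in opposite directions.
; On BeginPlay it finds and stores the BP_TableBase actor.
; Holding a key constrains the table's CubeComponent to the YZ plane and sets a fixed physics angular velocity around X.
; Releasing it restores the default constraint mode and zeroes the angular velocity.
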(event `Key|One`
  (params (Key :type "Key Structure"))
  ;[1 1 1] Rotate table
  (:`Pressed`
    (`PrimitiveComponent.SetConstraintMode` (`/Game/MyContent/BP_Table-Base.CubeComponent` (`self.Table`)) "YZPlane")
    (`PrimitiveComponent.SetPhysicsAngularVelocityInDegrees` (`/Game/MyContent/BP_Table-Base.CubeComponent` (`self.Table`)) (10.0 0.0 0.0) false "None"))
  (:`Released`
    (`PrimitiveComponent.SetConstraintMode` (`/Game/MyContent/BP_Table-Base.CubeComponent` (`self.Table`)) "Default")
    (`PrimitiveComponent.SetPhysicsAngularVelocityInDegrees` (`/Game/MyContent/BP_Table-Base.CubeComponent` (`self.Table`)) (0.0 0.0 0.0) false "None")))

(event `Key|Two`
  (params (Key :type "Key Structure"))
  ;[1 1 1] Rotate table
  (:`Pressed`
    (`PrimitiveComponent.SetConstraintMode` (`/Game/MyContent/BP_Table-Base.CubeComponent` (`self.Table`)) "YZPlane")
    (`PrimitiveComponent.SetPhysicsAngularVelocityInDegrees` (`/Game/MyContent/BP_Table-Base.CubeComponent` (`self.Table`)) (-10.0 0.0 0.0) false "None"))
  (:`Released`
    (`PrimitiveComponent.SetConstraintMode` (`/Game/MyContent/BP_Table-Base.CubeComponent` (`self.Table`)) "Default")
    (`PrimitiveComponent.SetPhysicsAngularVelocityInDegrees` (`/Game/MyContent/BP_Table-Base.CubeComponent` (`self.Table`)) (0.0 0.0 0.0) false "None")))

(event `self.ReceiveBeginPlay`
  (bind _returnvalue (`GameplayStatics.GetActorOfClass` "/Game/MyContent/BP_Table-Base.BP_Table-Base_C"))
  (set `self.Table` _returnvalue))

(fn `UserConstructionScript`)